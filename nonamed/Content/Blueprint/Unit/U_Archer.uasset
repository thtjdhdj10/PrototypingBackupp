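; Archer unit Blueprint that implements a ranged basic attack by firing arrow projectiles at its target.
; When attacking a valid target while active, it spawns an arrow, passes it the target, damage and owner, then plays a 2D attack sound.
; The launch direction aims above the target by the distance to it, angling the shot upward.
; Construction registers the Head in ColorBodies before running the parent script.
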(event `self.AttackTargetUnit`
  (bind _target (`self.Target`))
  (`/Engine/EditorBlueprintResources/StandardMacros.IsValid` (`self.Target`)
    (:`Is Valid`
      (bind _isactive (`self.CheckActive`))
      (if _isactive
        (bind _returnvalue (`|SpawnActorFromClass` "/Game/Blueprint/Projectile/Pr_Arrow_Blueprint.Pr_Arrow_Blueprint_C" (`KismetMathLibrary.MakeTransform` (.location (`self.GetTransform`)) (`KismetMathLibrary.Conv_VectorToRotator` (`KismetMathLibrary.GetDirectionUnitVector` (`self.K2_GetActorLocation`) (`KismetMathLibrary.MakeVector` (.x (`self.K2_GetActorLocation` _target)) (.y (`self.K2_GetActorLocation` _target)) (+ (.z (`self.K2_GetActorLocation` _target)) (`self.GetDistanceTo` _target))))) (.scale (`self.GetTransform`))) "Undefined" "OverrideRootScale"))
        (set `/Game/Blueprint/Projectile/Pr_Arrow_Blueprint.Target` (`self.Target`) _returnvalue)
        (set `/Game/Blueprint/Projectile/Pr_Arrow_Blueprint.ProjectileDamage` (`self.BasicAttackDamage`) _returnvalue)
        (set `/Game/Blueprint/Projectile/Pr_Arrow_Blueprint.ProjectileOwner` (`self.UnitOwner`) _returnvalue)
        (`GameplayStatics.PlaySound2D` "/Engine/EditorSounds/GamePreview/S_ProjectileAttackSound.S_ProjectileAttackSound")))))

(fn `UserConstructionScript`
  (set `self.ColorBodies` (`|MakeArray` (`self.Head`) :!type "Object Object Reference"))
  (`parent.UserConstructionScript`))