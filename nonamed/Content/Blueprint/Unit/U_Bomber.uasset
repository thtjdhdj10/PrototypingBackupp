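; U_Bomber is a unit that makes an area bomb attack on enemy units around it.
; AttackTargetUnit checks the target, then spawns a bomb effect at the bomber's own location and plays the attack sound.
; It then calls Damaged on every overlapping Unit with a different owner, passing zero rather than the unused BasicAttackDamage.
; The construction script registers Head in ColorBodies before running the parent's script.
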(event `self.AttackTargetUnit`
  (`/Engine/EditorBlueprintResources/StandardMacros.IsValid` (`self.Target`)
    (:`Is Valid`
      (bind _isactive (`self.CheckCorrectTarget`))
      (if _isactive
        (`|ExecutionSequence`
          (:`then_0`
            (`GameplayStatics.SpawnEmitterAtLocation` "/Game/KY_MagicEffects02/Particles/CP_BombAttack.CP_BombAttack" (`self.K2_GetActorLocation`))
            (`GameplayStatics.PlaySound2D` "/Engine/EditorSounds/GamePreview/S_BasicAttackSound.S_BasicAttackSound"))
          (:`then_1`
            (for _array_element (`self.GetOverlappingActors` "/Game/Blueprint/Unit/Unit.Unit_C")
              (bind _asunit (cast `/Game/Blueprint/Unit/Unit` _array_element))
              (if (not (`|EnumEquality` (`/Game/Blueprint/Unit/Unit.UnitOwner` _asunit) (`self.UnitOwner`)))
                (`self.Damaged` _asunit 0)))))))))

(fn `UserConstructionScript`
  (set `self.ColorBodies` (`|MakeArray` (`self.Head`) :!type "Object Object Reference"))
  (`parent.UserConstructionScript`))