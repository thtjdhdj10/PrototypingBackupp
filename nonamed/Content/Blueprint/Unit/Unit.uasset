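; Grid-based battle unit that players drag from a deck to deploy, with stats loaded from a DataTable by unit type.
; Clicking spawns a deck replacement and snaps the drag to deploy cells; release over the standby zone deploys within the population limit, and right-click releases it.
; UnitActivate picks a random nearest enemy, glides cell-to-cell through a Tick gate, then attacks on a timer if in range.
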(event `self.Capsule.OnComponentBeginOverlap`
  (params (OverlappedComponent :type "PrimitiveComponent Object Reference") (OtherActor :type "Actor Object Reference") (OtherComp :type "PrimitiveComponent Object Reference") (OtherBodyIndex :type Integer) (bFromSweep :type Boolean) (SweepResult :type "HitResult Structure (by ref)"))
  ;[1 1 1] Check Overlap Stage
  (cast `/Game/Blueprint/BP_BattleStandByZone` OtherActor)
  (set `self.isOverlapStandByZone` true))

(event `self.Capsule.OnComponentEndOverlap`
  (params (OverlappedComponent :type "PrimitiveComponent Object Reference") (OtherActor :type "Actor Object Reference") (OtherComp :type "PrimitiveComponent Object Reference") (OtherBodyIndex :type Integer))
  ;[1 1 1] Check Overlap Stage
  (cast `/Game/Blueprint/BP_BattleStandByZone` OtherActor)
  (set `self.isOverlapStandByZone` false))

(event `self.ReceiveTick`
  (params (DeltaSeconds :type "Float (single-precision)"))
  (bind _target (`self.Target`))
  (`|ExecutionSequence`
    (:`then_0`
      ;[1 1 1] Unit AI
      (if (`self.isActiveUnit`)
        (if (`self.isFight`)
          (`/Engine/EditorBlueprintResources/StandardMacros.IsValid` _target
            (:`Is Valid`
              (bind _isactive (`self.CheckCorrectTarget` _target))
              (if _isactive
                _))))
        (elif (not (`self.isFight`))
          ;[1 1 1] Drag to Unit Shift
          (`/Engine/EditorBlueprintResources/StandardMacros.Gate` true :!label _label
            (:`Exit`
              (bind _asplayer_controller (cast `PlayerController` (`Pawn.GetController` (`GameplayStatics.GetPlayerPawn` 0))))
              (bind (_worldlocation _worlddirection) (`PlayerController.DeprojectMousePositionToWorld` _asplayer_controller))
              (bind _returnvalue (/ (- 0.0 (.z _worldlocation)) (.z _worlddirection)))
              (bind _returnvalue_2 (+ (.x _worldlocation) (* (.x _worlddirection) _returnvalue)))
              (bind _returnvalue_3 (+ (.y _worldlocation) (* (.y _worlddirection) _returnvalue)))
              (bind (_indexedx _indexedy) (`/Game/Core/StaticFunction.WorldPosToIndexedPos` _returnvalue_2 _returnvalue_3))
              (bind _isvalid (`/Game/Core/StaticFunction.IsValidPosWithDeployZone` _indexedx _indexedy))
              (if _isvalid
                (bind (_worldx _worldy) (`/Game/Core/StaticFunction.IndexedPosToWorldPos` _indexedx _indexedy))
                (`self.K2_SetActorLocation` (`KismetMathLibrary.MakeVector` _worldx _worldy))
                (else
                  (`self.K2_SetActorLocation` (`KismetMathLibrary.MakeVector` _returnvalue_2 _returnvalue_3)))))))))
    (:`then_1`
      (`SceneComponent.K2_SetWorldRotation` (`self.hpBar_Widget`) (struct :`Yaw` 180.0) false false))
    (:`then_2`
      (`/Engine/EditorBlueprintResources/StandardMacros.Gate` true :!label _label_2
        (:`Exit`
          (`self.K2_SetActorLocation` (`KismetMathLibrary.MakeVector` (+ (* DeltaSeconds (`self.moveSpeedX`)) (.x (`self.K2_GetActorLocation`))) (+ (* DeltaSeconds (`self.moveSpeedY`)) (.y (`self.K2_GetActorLocation`))) (.z (`self.K2_GetActorLocation`)))))))))

(event `self.ReceiveBeginPlay`
  ;[1 1 1] Init
  (`|ExecutionSequence`
    (:`then_0`
      ;[1 1 1] Check Overlap Stage
      (set `self.isOverlapStandByZone` (>= (`KismetArrayLibrary.Array_Length` (`PrimitiveComponent.GetOverlappingActors` (`self.Capsule`) "/Game/Blueprint/BP_BattleStandByZone.BP_BattleStandByZone_C")) 1)))
    (:`then_1`
      (if (not (`self.isActiveUnit`))
        (`self.EnableInput` (`GameplayStatics.GetPlayerController` 0))))
    (:`then_2`
      (`self.SetUnitColor`))
    (:`then_3`
      (bind _asw_unit_state (cast `/Game/Widget/W_UnitState` (`WidgetComponent.GetUserWidgetObject` (`self.hpBar_Widget`))))
      (set `/Game/Widget/W_UnitState.ownerUnit` self _asw_unit_state))
    (:`then_4`
      (`self.SetIndexedLocation`))))

(event `Damaged`
  (params (damage :type Integer))
  ;[1 1 1] Damaged
  (`self.DecreaseHP` damage)
  (`self.SetMaterial` "/Game/Material/M_DamagedUnitColor.M_DamagedUnitColor")
  (`KismetSystemLibrary.Delay` 0.2)
  (`self.SetUnitColor`))

(event `MoveStart`
  (goto _label_2 :!via `Open`))

(event `StopMove`
  (`self.SetIndexedLocation`)
  (goto _label_2 :!via `Close`))

(event `self.ReceiveActorOnClicked`
  (params (ButtonPressed :type "Key Structure" :default "AnyKey"))
  ;[1 1 1] Drag to Unit Shift
  (bind _asplayer_bp (cast `/Game/Core/PlayerBP` (`GameplayStatics.GetPlayerPawn` 0)))
  (if (`|EnumEquality` (`/Game/Core/PlayerBP.GameState` _asplayer_bp) "NewEnumerator0")
    (if (not (`self.isActiveUnit`))
      (set `self.isDeckUnit` false)
      (`self.CopyUnit`)
      (goto _label :!via `Open`))))

(event `InputAction|Mouse Right Button Click` :consume false
  (params (Key :type "Key Structure" :default "AnyKey"))
  ;[1 1 1] Right Click to Release Deployed Unit
  (:`Pressed`
    (if (`|EnumEquality` (`self.UnitOwner`) "NewEnumerator1")
      (if (`self.isActiveUnit`)
        (if (`self.isFight`)
          _
          (elif (== (`.HitComponent` (`GameplayStatics.BreakHitResult` (`PlayerController.GetHitResultUnderCursorByChannel` (`GameplayStatics.GetPlayerController` 0) "TraceTypeQuery1" true))) (`self.Capsule`))
            (`self.ReleaseDeployedUnit`)))))))

(event `self.ReceiveDestroyed`
  (`GameplayStatics.PlaySound2D` "/Game/S_unit_die.S_unit_die"))

(event `InputAction|Mouse Left Button Click` :consume false
  (params (Key :type "Key Structure" :default "AnyKey"))
  ;[1 1 1] Drag to Unit Shift
  (:`Released`
    (bind _asplayer_bp (cast `/Game/Core/PlayerBP` (`GameplayStatics.GetPlayerPawn` 0)))
    (if (`|EnumEquality` (`/Game/Core/PlayerBP.GameState` _asplayer_bp) "NewEnumerator0")
      (`|ExecutionSequence`
        (:`then_0`
          (goto _label :!via `Close`))
        (:`then_1`
          (if (`|EnumEquality` (`self.UnitOwner`) "NewEnumerator0")
            (if (`self.isActiveUnit`)
              _
              (elif (`self.isOverlapStandByZone`)
                (`self.DeployUnit`)
                (`self.SetUnitColor`)
                (`GameplayStatics.SpawnEmitterAtLocation` "/Game/KY_MagicEffects03/Particles/P_UnitDeployEffect.P_UnitDeployEffect" (`self.K2_GetActorLocation`))
                (`GameplayStatics.SpawnSound2D` "/Engine/VREditor/Sounds/VR_teleport.VR_teleport")
                (elif (not (`self.isDeckUnit`))
                  (`self.DeployCanceld`))))))))))

(fn `AttackTargetUnit`
  (bind _target (`self.Target`))
  (`GameplayStatics.SpawnEmitterAtLocation` "/Game/KY_MagicEffects02/Particles/CP_impact4.CP_impact4" (`self.K2_GetActorLocation` _target) (struct))
  (`self.Damaged` _target (`self.iAttackDamage`))
  (`GameplayStatics.PlaySound2D` "/Engine/EditorSounds/GamePreview/S_BasicAttackSound.S_BasicAttackSound"))

(fn `CheckAttackDelay`
  (params (deltaTime :type "Float (double-precision)"))
  (returns (isAttackCharge :type Boolean))
  (bind _attackdelaydeltapercent (`self.AttackDelayDeltaPercent`))
  (`/Engine/EditorBlueprintResources/StandardMacros.IsValid` (`self.Target`)
    (:`Is Valid`
      (bind _isactive (`self.CheckCorrectTarget`))
      (if _isactive
        (if (<= (`self.CurrentAttackDelay`) 0.0)
          (set `self.CurrentAttackDelay` (* (+ (`KismetMathLibrary.RandomFloatInRange` (* -1.0 _attackdelaydeltapercent) _attackdelaydeltapercent) 1.0) (`self.AttackDelay`)))
          (return true)
          (else
            (set `self.CurrentAttackDelay` (- (`self.CurrentAttackDelay`) deltaTime))
            (return false)))
        (else
          _)))
    (:`Is Not Valid`
      _))
  (return false))

(fn `CheckAttackTarget`
  (returns (isCorrectAttackTarget :type Boolean))
  (bind _isactive (`self.CheckCorrectTarget`))
  (if _isactive
    (bind _istargetinrange (`/Game/Core/StaticFunction.CheckTargetUnitInRange` self (`self.Target`)))
    (return _istargetinrange)
    (else
      (return false))))

(fn `CheckBattle`
  (returns (isFight :type Boolean))
  (if (`self.isActiveUnit`)
    (if (`self.isFight`)
      (return true)
      (else
        _)))
  (return false))

(fn `CheckCorrectEnemy`
  (params (targetUnit :type "/Game/Blueprint/Unit/Unit Object Reference"))
  (returns (isCorrectEnemy :type Boolean))
  (`/Engine/EditorBlueprintResources/StandardMacros.IsValid` targetUnit
    (:`Is Valid`
      (if (`|EnumEquality` (`self.UnitOwner`) (`/Game/Blueprint/Unit/Unit.UnitOwner` targetUnit))
        _
        (elif (`/Game/Blueprint/Unit/Unit.isActiveUnit` targetUnit)
          (if (`/Game/Blueprint/Unit/Unit.isFight` targetUnit)
            (return true)
            (else
              _)))))
    (:`Is Not Valid`
      _))
  (return false))

(fn `CheckCorrectTarget`
  (returns (isActive :type Boolean))
  (bind _target (`self.Target`))
  (`/Engine/EditorBlueprintResources/StandardMacros.IsValid` _target
    (:`Is Valid`
      (if (`/Game/Blueprint/Unit/Unit.isActiveUnit` _target)
        (if (`/Game/Blueprint/Unit/Unit.isFight` _target)
          (return true)
          (else
            _))))
    (:`Is Not Valid`
      _))
  (return false))

(fn `CheckNearestDisRange`
  (returns (isTargetInRange :type Boolean))
  (set `self.NearestOppDis` (`self.GetDistanceTo` (`self.Target`)))
  (return (<= (`self.NearestOppDis`) (`self.AttackRange`))))

(fn `CopyUnit`
  (bind _returnvalue (`|SpawnActorFromClass` (`GameplayStatics.GetObjectClass` self) (`KismetMathLibrary.MakeTransform` (`self.K2_GetActorLocation`) (struct) (1.0 1.0 1.0)) "Undefined" "OverrideRootScale"))
  (`self.SetActive` _returnvalue false)
  (set `/Game/Blueprint/Unit/Unit.isDeckUnit` true _returnvalue))

(fn `CountSearchTargetFrame`
  (returns (isSearchingFrame :type Boolean))
  (if (>= (`self.CurrentSearchTargetDelayFrame`) 0)
    (set `self.CurrentSearchTargetDelayFrame` (+ (`self.CurrentSearchTargetDelayFrame`) -1))
    (return false)
    (else
      (bind _output_get (set `self.SearchTargetDelayFrame` (`KismetMathLibrary.RandomIntegerInRange` (`self.MinSearchTargetDelayFrame`) (`self.MaxSearchTargetDelayFrame`))))
      (set `self.CurrentSearchTargetDelayFrame` _output_get)
      (return true))))

(fn `DecreaseHP`
  (params (decreaseFactor :type Integer))
  (bind _output_get (set `self.iCurrentHP` (- (`self.iCurrentHP`) decreaseFactor)))
  (if (<= _output_get 0)
    (`self.K2_DestroyActor`)))

(fn `DeployCanceld`
  (`self.K2_DestroyActor`))

(fn `DeployUnit`
  (bind _population (`self.population`))
  (`self.SetIndexedLocation`)
  (bind _asplayer_bp (cast `/Game/Core/PlayerBP` (`GameplayStatics.GetPlayerPawn` 0)))
  (bind _currentusingpopulation (`/Game/Core/PlayerBP.currentUsingPopulation` _asplayer_bp))
  (if (>= (- (`/Game/Core/PlayerBP.maxPopulation` _asplayer_bp) _currentusingpopulation) _population)
    (set `/Game/Core/PlayerBP.currentUsingPopulation` (+ _currentusingpopulation _population) _asplayer_bp)
    (`self.SetActive` true)
    (set `self.UnitOwner` "NewEnumerator1")
    (else
      (`self.DeployCanceld`))))

(fn `MoveTargetPosition`
  (params (targetX :type Integer) (targetY :type Integer) (duration :type "Float (double-precision)"))
  (bind (_worldx _worldy) (`/Game/Core/StaticFunction.IndexedPosToWorldPos` targetX targetY))
  (bind (_worldx_2 _worldy_2) (`/Game/Core/StaticFunction.IndexedPosToWorldPos` (`self.xPos`) (`self.yPos`)))
  (set `self.moveSpeedX` (/ (- _worldx _worldx_2) duration))
  (set `self.moveSpeedY` (/ (- _worldy _worldy_2) duration))
  (`self.MoveStart`)
  (`KismetSystemLibrary.K2_SetTimer` null "StopMove" duration))

(fn `MoveToTargetUnit`
  (params (deltaTime :type "Float (double-precision)"))
  (bind _location (.location (`self.GetTransform`)))
  (set `self.moveDistance` (* deltaTime (`self.MoveSpeed`)))
  (`/Engine/EditorBlueprintResources/StandardMacros.IsValid` (`self.Target`)
    (:`Is Valid`
      (bind _isactive (`self.CheckCorrectTarget`))
      (if _isactive
        (bind _output_get (set `self.moveDelta` (* (`KismetMathLibrary.GetDirectionUnitVector` _location (.location (`self.GetTransform` (`self.Target`)))) (`self.moveDistance`))))
        (bind _sweephitresult (`self.K2_SetActorTransform` (`KismetMathLibrary.MakeTransform` (+ _location (`self.moveDelta`)) (`KismetMathLibrary.Conv_VectorToRotator` _output_get) (.scale (`self.GetTransform`))) true))
        (bind (_bblockinghit _binitialoverlap _time _location_2 _impactpoint _normal _impactnormal _physmat _hitactor) (`GameplayStatics.BreakHitResult` _sweephitresult))
        (if _bblockinghit
          (bind _output_get_2 (set `self.moveDelta` (* (`KismetMathLibrary.GetDirectionUnitVector` (`self.K2_GetActorLocation` _hitactor) (`self.K2_GetActorLocation`)) (`self.moveDistance`))))
          (`self.K2_SetActorLocation` (+ _output_get_2 _location) true))
        ;[1 1 1] Z 는 항상 0
        (`self.K2_SetActorLocation` (`KismetMathLibrary.MakeVector` (.x (`self.K2_GetActorLocation`)) (.y (`self.K2_GetActorLocation`))))))))

(fn `ReleaseDeployedUnit`
  (bind _asplayer_bp (cast `/Game/Core/PlayerBP` (`GameplayStatics.GetPlayerPawn` 0)))
  (set `/Game/Core/PlayerBP.currentUsingPopulation` (`KismetMathLibrary.Max` (- (`/Game/Core/PlayerBP.currentUsingPopulation` _asplayer_bp) (`self.population`))) _asplayer_bp)
  (`self.K2_DestroyActor`))

(fn `SearchTarget`
  (returns (searched :type Boolean))
  (locals (correctMinDisTargetArr :type "Array of /Game/Blueprint/Unit/Unit Object Reference") (minDistance :type Integer :default 9999))
  (bind _mindistance (`local.minDistance`))
  (bind _correctmindistargetarr (`local.correctMinDisTargetArr`))
  (bind _correctmindistargetarr_2 (`local.correctMinDisTargetArr`))
  (bind _returnvalue (`KismetArrayLibrary.Array_Length` _correctmindistargetarr))
  (bind _outactors (`GameplayStatics.GetAllActorsOfClass` "Unit_C"))
  ;[1 1 1] 가장 가까운 적들을 Arr에
  (for _array_element _outactors
    (bind _iscorrectenemy (`self.CheckCorrectEnemy` self _array_element))
    (if _iscorrectenemy
      (bind _distance (`/Game/Core/StaticFunction.GetDistanceWithUnit` self _array_element))
      (if (< _distance _mindistance)
        (`KismetArrayLibrary.Array_Clear` _correctmindistargetarr_2)
        (`KismetArrayLibrary.Array_Add` _correctmindistargetarr_2 _array_element)
        (elif (== _distance _mindistance)
          (`KismetArrayLibrary.Array_Add` _correctmindistargetarr_2 _array_element)))))
  (if (== _returnvalue 0)
    (return false)
    (else
      (set `self.Target` (`KismetArrayLibrary.Array_Get` _correctmindistargetarr (`KismetMathLibrary.RandomIntegerInRange` 0 (- _returnvalue 1))))
      (return true))))

(fn `SetActive`
  (params (active :type Boolean))
  (`|ExecutionSequence`
    (:`then_0`
      (set `self.isActiveUnit` active)
      (for _array_element (`self.ColorBodies`)
        (bind _asstatic_mesh_component (cast `StaticMeshComponent` _array_element))
        (`PrimitiveComponent.SetRenderCustomDepth` _asstatic_mesh_component (not active))
        (`|CreateWidget` "/Game/Widget/W_UnitState.W_UnitState_C")))))

(fn `SetIndexedLocation`
  (bind (_indexedx _indexedy) (`/Game/Core/StaticFunction.WorldPosToIndexedPos` (.x (`self.K2_GetActorLocation`)) (.y (`self.K2_GetActorLocation`))))
  (bind _output_get (set `self.xPos` _indexedx))
  (bind _output_get_2 (set `self.yPos` _indexedy))
  (bind (_worldx _worldy) (`/Game/Core/StaticFunction.IndexedPosToWorldPos` _output_get _output_get_2))
  (`self.K2_SetActorLocation` (`KismetMathLibrary.MakeVector` _worldx _worldy)))

(fn `SetMaterial`
  (params (mat :type "Material Object Reference"))
  (for _array_element (`self.ColorBodies`)
    (bind _asstatic_mesh_component (cast `StaticMeshComponent` _array_element))
    (`PrimitiveComponent.SetMaterial` _asstatic_mesh_component 0 mat)))

(fn `SetMaterialScalarValue`
  (params (paramName :type Name) (scalarFactor :type "Float (double-precision)"))
  (for _array_element (`self.ColorBodies`)
    (bind _asmesh_component (cast `MeshComponent` _array_element))
    (`MeshComponent.SetScalarParameterValueOnMaterials` _asmesh_component paramName scalarFactor))
  (return))

(fn `SetUnitColor`
  (switch `/Game/Type/Owner` (`self.UnitOwner`)
    (:`NewEnumerator1`
      (`self.SetMaterial` "/Game/Material/M_PlayerUnitColor.M_PlayerUnitColor"))
    (:`NewEnumerator2`
      (`self.SetMaterial` "/Game/Material/M_OpponentUnitColor.M_OpponentUnitColor"))))

(fn `SetUnitStatus`
  (params (inputUnitType :type "/Game/Type/UnitType Enum"))
  (locals (targetStatus :type "/Game/Type/UnitStatus Structure"))
  (bind (_maxhp _attackdamage _attackrange _attackprevdelay _moverange _moveprevdelay _population _siegedamage) (break `/Game/Type/UnitStatus` (`local.targetStatus`)))
  (switch `/Game/Type/UnitType` inputUnitType
    (:`NewEnumerator1`
      (bind _returnvalue (`|GetDataTableRow` "/Game/UnitStatusDatatable.UnitStatusDatatable" "Knight")
        (:`then`
          (set `local.targetStatus` _returnvalue))))
    (:`NewEnumerator2`
      (bind _returnvalue_2 (`|GetDataTableRow` "/Game/UnitStatusDatatable.UnitStatusDatatable" "MiniKnight")
        (:`then`
          (set `local.targetStatus` _returnvalue_2))))
    (:`NewEnumerator3`
      (bind _returnvalue_3 (`|GetDataTableRow` "/Game/UnitStatusDatatable.UnitStatusDatatable" "GiantKnight")
        (:`then`
          (set `local.targetStatus` _returnvalue_3))))
    (:`NewEnumerator4`
      (bind _returnvalue_4 (`|GetDataTableRow` "/Game/UnitStatusDatatable.UnitStatusDatatable" "Archer")
        (:`then`
          (set `local.targetStatus` _returnvalue_4))))
    (:`NewEnumerator5`
      (bind _returnvalue_5 (`|GetDataTableRow` "/Game/UnitStatusDatatable.UnitStatusDatatable" "Bomber")
        (:`then`
          (set `local.targetStatus` _returnvalue_5))))
    (:`NewEnumerator6`
      (bind _returnvalue_6 (`|GetDataTableRow` "/Game/UnitStatusDatatable.UnitStatusDatatable" "MiniArcher")
        (:`then`
          (set `local.targetStatus` _returnvalue_6)))))
  (set `self.SiegeDamage` _siegedamage)
  (set `self.population` _population)
  (set `self.movePrevDelay` _moveprevdelay)
  (set `self.iMoveDistance` _moverange)
  (set `self.iAttackPrevDelay` _attackprevdelay)
  (set `self.iAttackRange` _attackrange)
  (set `self.iAttackDamage` _attackdamage)
  (set `self.iMaxHP` _maxhp)
  (set `self.iCurrentHP` (`self.iMaxHP`)))

(fn `UnitActivate`
  (bind _searched (`self.SearchTarget`))
  (if _searched
    (bind _nearestpos (`/Game/Core/StaticFunction.GetNearestMovePos` self (`self.Target`)))
    (bind (_x _y) (break `/Game/Type/IntVector2` _nearestpos))
    (`self.MoveTargetPosition` _x _y 1.25)
    (set `self.xPos` _x)
    (set `self.yPos` _y)
    (bind _iscorrectattacktarget (`self.CheckAttackTarget`))
    (if _iscorrectattacktarget
      (`KismetSystemLibrary.K2_SetTimer` null "AttackTargetUnit" 1.5))))

(fn `UserConstructionScript`
  (`self.SetUnitStatus` (`self.unitType`))
  (for _array_element (`self.ColorBodies`)
    (bind _asstatic_mesh_component (cast `StaticMeshComponent` _array_element))
    (`PrimitiveComponent.SetRenderCustomDepth` _asstatic_mesh_component false)))