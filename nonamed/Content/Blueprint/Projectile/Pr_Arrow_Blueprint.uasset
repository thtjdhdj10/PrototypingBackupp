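; Homing arrow projectile that damages its target unit.
; Tick locks the homing component onto the Target once and destroys the arrow if the Target becomes invalid or the arrow drops to ground level.
; After a short delay, capsule overlap with a unit of another owner also destroys it.
; Damage is applied in Destroyed, so every destruction calls damage on the stored Target, with impact particles and sound.
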(event `self.ReceiveDestroyed`
  (`/Game/Blueprint/Unit/Unit.Damaged` (`self.Target`) (`self.ProjectileDamage`))
  (`GameplayStatics.SpawnEmitterAtLocation` "/Game/KY_MagicEffects02/Particles/CP_impact4.CP_impact4" (`self.K2_GetActorLocation`))
  (`GameplayStatics.PlaySound2D` "/Engine/EditorSounds/GamePreview/S_BasicAttackSound.S_BasicAttackSound"))

(event `self.ReceiveTick`
  (params (DeltaSeconds :type "Float (single-precision)"))
  (bind _target (`self.Target`))
  (`/Engine/EditorBlueprintResources/StandardMacros.IsValid` (`self.Target`)
    (:`Is Valid`
      (`|ExecutionSequence`
        (:`then_0`
          (`/Engine/EditorBlueprintResources/StandardMacros.DoOnce` false
            (:`Completed`
              (`/Engine/EditorBlueprintResources/StandardMacros.IsValid` _target
                (:`Is Valid`
                  (set `ProjectileMovementComponent.HomingTargetComponent` (`self.K2_GetRootComponent` _target) (`self.Projectile`)))))))
        (:`then_1`
          (if (<= (.z (`self.K2_GetActorLocation`)) 0.0)
            (`self.K2_DestroyActor`)))))
    (:`Is Not Valid`
      (`self.K2_DestroyActor`))))

(event `self.Capsule.OnComponentBeginOverlap`
  (params (OverlappedComponent :type "PrimitiveComponent Object Reference") (OtherActor :type "Actor Object Reference") (OtherComp :type "PrimitiveComponent Object Reference") (OtherBodyIndex :type Integer) (bFromSweep :type Boolean) (SweepResult :type "HitResult Structure (by ref)"))
  (`KismetSystemLibrary.Delay` 0.02)
  (if (`KismetMathLibrary.ClassIsChildOf` (`GameplayStatics.GetObjectClass` OtherActor) "/Game/Blueprint/Unit/Unit.Unit_C")
    (bind _asunit (cast `/Game/Blueprint/Unit/Unit` OtherActor))
    (if (`|EnumInequality` (`/Game/Blueprint/Unit/Unit.UnitOwner` _asunit) (`self.ProjectileOwner`))
      (`self.K2_DestroyActor`))))

(fn `UserConstructionScript`)