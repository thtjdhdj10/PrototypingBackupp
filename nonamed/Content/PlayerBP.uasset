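; Player Blueprint that runs the game flow of a unit-deck battler with deploy, battle, result and unit-selection phases.
; BeginPlay fills the selectable unit pool and opens the UI; GoNextGameSteb advances GameState, swaps phase widgets and starts battles via MyGameBase.
; Helpers map unit types to classes, images and population, draw random units out of the pool, and spawn inactive units into six deck slots.
; Battle end and win events only print messages.
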(event `self.ReceiveBeginPlay`
  (bind _returnvalue (`GameplayStatics.GetPlayerController` 0))
  (set `PlayerController.bShowMouseCursor` true _returnvalue)
  (set `PlayerController.bEnableClickEvents` true _returnvalue)
  (bind _enumvalue (foreach `/Game/Type/UnitType`)
    (:`LoopBody`
      (bind _unit (`self.UnitTypeToUnitBP` _enumvalue))
      (`KismetArrayLibrary.Array_Add` (`self.SelectableUnit`) _unit))
    (:`then`
      (set `self.GameState` "NewEnumerator0")
      (bind _returnvalue_2 (`|CreateWidget` "/Game/Widget/W_DeployUnit.W_DeployUnit_C"))
      (`UserWidget.AddToViewport` _returnvalue_2 0)
      (set `self.CurrentWidget` _returnvalue_2)
      (`self.AddUnitToDeck` "NewEnumerator3")
      (bind _returnvalue_3 (`|CreateWidget` "/Game/Widget/W_GameStatement.W_GameStatement_C"))
      (`UserWidget.AddToViewport` _returnvalue_3 0)
      (set `/Game/Widget/W_GameStatement.player` self _returnvalue_3))))

(event `PlayerWin`
  (`KismetSystemLibrary.PrintString` "Player Win"))

(event `OpponentWin`
  (`KismetSystemLibrary.PrintString` "Opponent Win"))

(fn `AddUnitToDeck`
  (params (unitType :type "/Game/Type/UnitType Enum"))
  (bind _selectunitcount (`self.selectUnitCount`))
  (if (not (>= _selectunitcount 6))
    (`KismetArrayLibrary.Array_Add` (`self.PlayerUnitDeck`) unitType)
    (bind _unit (`self.UnitTypeToUnitBP` unitType))
    (bind _returnvalue (`|SpawnActorFromClass` _unit (`KismetMathLibrary.MakeTransform` (`self.K2_GetActorLocation` (`KismetArrayLibrary.Array_Get` (`/Game/Player_Deck_Blueprint.unitDeckArr` (`self.deck`)) _selectunitcount))) "Undefined" "OverrideRootScale"))
    (`GameplayStatics.SpawnEmitterAtLocation` "/Game/KY_MagicEffects03/Particles/P_UnitGenerate.P_UnitGenerate" (`self.K2_GetActorLocation` _returnvalue))
    (`GameplayStatics.SpawnSound2D` "/Engine/EditorSounds/GamePreview/PossessPlayer.PossessPlayer")
    (set `/Game/Blueprint/Unit/Unit.isDeckUnit` true _returnvalue)
    (`/Game/Blueprint/Unit/Unit.SetActive` _returnvalue false)
    (`/Engine/EditorBlueprintResources/StandardMacros.IncrementInt` (`self.selectUnitCount`))))

(fn `BattleEnd`
  (params (winner :type "/Game/Type/Owner Enum") (restUnitPopulation :type Integer))
  (switch `/Game/Type/Owner` winner
    (:`NewEnumerator1`
      (set `self.winner` "NewEnumerator1")
      (`KismetSystemLibrary.PrintString` (`KismetStringLibrary.BuildString_Int` (`KismetStringLibrary.Conv_NameToString` (`|GetEnumeratorName` (enumliteral `/Game/Type/Owner` "NewEnumerator2"))) " Damaged: " restUnitPopulation " !")))
    (:`NewEnumerator2`
      (set `self.winner` "NewEnumerator2")
      (`KismetSystemLibrary.PrintString` (`KismetStringLibrary.BuildString_Int` (`KismetStringLibrary.Conv_NameToString` (`|GetEnumeratorName` (enumliteral `/Game/Type/Owner` "NewEnumerator1"))) " Damaged: " restUnitPopulation " !")))))

(fn `GetActorNearHand`
  (returns (NearestMesh :type "Actor Object Reference")))

(fn `GetSelectableUnit`
  (params (count :type Integer))
  (returns (unitArray :type "Array of /Game/Blueprint/Unit/Unit Class Reference"))
  (bind _selectableunit (`self.SelectableUnit`))
  (bind _selectableunit_2 (`self.SelectableUnit`))
  (`KismetArrayLibrary.Array_Clear` (`self.retSelectableUnit`))
  (if (>= count (`KismetArrayLibrary.Array_Length` (`self.SelectableUnit`)))
    (set `self.retSelectableUnit` _selectableunit)
    (`KismetArrayLibrary.Array_Clear` _selectableunit)
    (return (`self.retSelectableUnit`))
    (else
      (while (> count (`KismetArrayLibrary.Array_Length` (`self.retSelectableUnit`)))
        (bind _output_get (set `self.randomInteger` (`KismetMathLibrary.RandomIntegerInRange` 0 (- (`KismetArrayLibrary.Array_Length` (`self.SelectableUnit`)) 1))))
        (bind _item (`KismetArrayLibrary.Array_Get` _selectableunit_2 _output_get))
        (`KismetArrayLibrary.Array_Add` (`self.retSelectableUnit`) _item)
        (`KismetArrayLibrary.Array_RemoveItem` _selectableunit_2 _item))
      (return (`self.retSelectableUnit`)))))

(fn `GoNextGameSteb`
  (bind _asuser_widget (cast `UserWidget` (`self.CurrentWidget`))
    (:`then`
      (`Widget.RemoveFromParent` _asuser_widget)
      (switch `/Game/Type/GameFlowStatement` (`self.GameState`)
        (:`NewEnumerator0`
          (set `self.GameState` "NewEnumerator7")
          (bind _returnvalue (`|CreateWidget` "/Game/Widget/W_Battle.W_Battle_C"))
          (set `self.CurrentWidget` _returnvalue)
          (bind _asmy_game_base (cast `/Game/MyGameBase` (`GameplayStatics.GetGameState`))
            (:`then`
              (`/Game/MyGameBase.BattleStart` _asmy_game_base))
            (:`CastFailed`
              _)))
        (:`NewEnumerator7`
          (set `self.GameState` "NewEnumerator9")
          (bind _returnvalue_2 (`|CreateWidget` "/Game/Widget/W_BattleResult.W_BattleResult_C"))
          (set `self.CurrentWidget` _returnvalue_2))
        (:`NewEnumerator9`
          (if (`self.isPlayerSelectTurn`)
            (set `self.GameState` "NewEnumerator3")
            (bind _returnvalue_3 (`|CreateWidget` "/Game/Widget/W_SelectUnit.W_SelectUnit_C"))
            (set `self.CurrentWidget` _returnvalue_3)
            (set `self.isPlayerSelectTurn` (not (`self.isPlayerSelectTurn`)))
            (else
              (set `self.GameState` "NewEnumerator1")
              (bind _returnvalue_4 (`|CreateWidget` "/Game/Widget/W_OpponentSelection.W_OpponentSelection_C"))
              (set `self.CurrentWidget` _returnvalue_4))))
        (:`NewEnumerator1`
          (set `self.GameState` "NewEnumerator0" :!label _label)
          (bind _returnvalue_5 (`|CreateWidget` "/Game/Widget/W_DeployUnit.W_DeployUnit_C"))
          (set `self.CurrentWidget` _returnvalue_5))
        (:`NewEnumerator3`
          (goto _label)))
      (`UserWidget.AddToViewport` _returnvalue 0)
      (`UserWidget.AddToViewport` _returnvalue_2 0)
      (`UserWidget.AddToViewport` _returnvalue_3 0)
      (`UserWidget.AddToViewport` _returnvalue_5 0)
      (`UserWidget.AddToViewport` _returnvalue_4 0)
      (return))
    (:`CastFailed`
      (return))))

(fn `UnitTypeToPopulation`
  (params (type :type "/Game/Type/UnitType Enum"))
  (returns (population :type Integer))
  (bind _unit (`self.UnitTypeToUnitBP` type))
  (return (`.population` (defaults `/Game/PlayerBP` _unit))))

(fn `UnitTypeToUnitBP`
  (params (NewParam :type "/Game/Type/UnitType Enum"))
  (returns (unit :type "/Game/Blueprint/Unit/Unit Class Reference"))
  (switch `/Game/Type/UnitType` NewParam
    (:`NewEnumerator1`
      (set `self.retUnit` "/Game/Blueprint/Unit/U_Knight.U_Knight_C"))
    (:`NewEnumerator2`
      (set `self.retUnit` "/Game/Blueprint/Unit/U_MiniKnight.U_MiniKnight_C"))
    (:`NewEnumerator3`
      (set `self.retUnit` "/Game/Blueprint/Unit/U_GiantKnight.U_GiantKnight_C"))
    (:`NewEnumerator4`
      (set `self.retUnit` "/Game/Blueprint/Unit/U_Archer.U_Archer_C"))
    (:`NewEnumerator5`
      (set `self.retUnit` "/Game/Blueprint/Unit/U_Bomber.U_Bomber_C"))
    (:`NewEnumerator6`
      (set `self.retUnit` "/Game/Blueprint/Unit/U_MiniArcher.U_MiniArcher_C")))
  (return (`self.retUnit`)))

(fn `UnitTypeToUnitImage`
  (params (unitType :type "/Game/Type/UnitType Enum"))
  (returns (image :type "Texture Object Reference"))
  (switch `/Game/Type/UnitType` unitType
    (:`NewEnumerator1`
      (set `self.retImage` "/Game/Textures/T_knight.T_knight"))
    (:`NewEnumerator2`
      (set `self.retImage` "/Game/Textures/T_miniknight.T_miniknight"))
    (:`NewEnumerator3`
      (set `self.retImage` "/Game/Textures/T_giantknight.T_giantknight"))
    (:`NewEnumerator4`
      (set `self.retImage` "/Game/Textures/T_archer.T_archer"))
    (:`NewEnumerator5`
      (set `self.retImage` "/Game/Textures/T_bomber.T_bomber"))
    (:`NewEnumerator6`
      (set `self.retImage` "/Game/Textures/T_miniarcher.T_miniarcher")))
  (return (`self.retImage`)))

(fn `UserConstructionScript`
  (set `self.currentPlayerHP` (`self.playerHPmax`))
  (set `self.currentOpponentHP` (`self.opponentHPmax`)))